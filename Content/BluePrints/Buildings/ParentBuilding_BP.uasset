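; ParentBuilding_BP is a building Blueprint, named as a parent class, that animates a vertical rise for smooth construction.
; RiseBuilding calls the Rise dispatcher, which is bound to the Rise event on BeginPlay and unbound on EndPlay.
; A timeline then lerps the actor's Z toward RiseZ from its current height each update, rather than a cached start, keeping X and Y unchanged.
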(event `self.ReceiveBeginPlay`
  (add `self.Rise_Dispatcher` (delegate `Event Rise`)))

(event `Event Rise`
  ;[1 1 1] For Smooth Construct
  (bind (_direction _float_output) (`Timeline|Rise_Timeline`)
    (:`Update`
      (`self.K2_SetActorLocation` (`KismetMathLibrary.MakeVector` (.x (`self.K2_GetActorLocation`)) (.y (`self.K2_GetActorLocation`)) (`KismetMathLibrary.Lerp` (.z (`self.K2_GetActorLocation`)) (`self.RiseZ`) _float_output))))))

(event `self.ReceiveEndPlay`
  (params (EndPlayReason :type "EEndPlayReason Enum" :default "Destroyed"))
  (remove `self.Rise_Dispatcher` (delegate `Event Rise`)))

(fn `RiseBuilding`
  (`self.Rise_Dispatcher`))

(fn `UserConstructionScript`)